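; AC_Interaction is an interaction component that outlines the actor the player targets and switches input mappings around interaction.
; UpdateInteractState outlines the current hit actor, clears the previous one and adds IMC_Default through AC_InputControls on the player character.
; Without a hit it only clears the previous outline.
; TriggerInteract runs the parent logic, then removes IMC_Interact through AC_InputControls on the player controller.
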(fn UpdateInteractState
  (params (bHit :type Boolean))
  (if bHit
    (Class|BPIInteractOLD|SetOutlineState(Message) (Variables|Default|GetCurrentHitActor) true)
    (Utilities|IsValid (Variables|Default|GetPrevouseHitActor)
      (:Is%20Valid
        (Class|BPIInteractOLD|SetOutlineState(Message) (Variables|Default|GetPrevouseHitActor) false))
      (:Is%20Not%20Valid
        _))
    (Default|AddInputMapping (Actor|GetComponentbyClass (Game|GetPlayerCharacter 0) "/Game/Junk/Components/AC_InputControls.AC_InputControls_C") "/Game/ThirdPerson/Input/IMC_Default.IMC_Default")
    (else
      (Utilities|IsValid (Variables|Default|GetPrevouseHitActor)
        (:Is%20Valid
          (Class|BPIInteractOLD|SetOutlineState(Message) (Variables|Default|GetPrevouseHitActor) false))))))

(fn TriggerInteract
  (|CallParentFunction)
  (Input|RemoveMappingContext (Actor|GetComponentbyClass (Game|GetPlayerController 0) "/Game/Junk/Components/AC_InputControls.AC_InputControls_C") "/Game/ThirdPerson/Input/IMC_Interact.IMC_Interact" "(bIgnoreAllPressedKeysUntilRelease=True,bForceImmediately=False,bNotifyUserSettings=False)"))