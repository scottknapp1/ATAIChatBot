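; Actor component that serves as the core of an interaction system, detecting interactable actors at screen center and triggering hold-to-interact.
; A line trace, run per tick or on a looping timer, extends by interact distance plus camera-to-owner distance.
; Hit changes reset hold progress and call UpdateInteractState, an empty hook here.
; UpdateInteract compares hold duration to the target's required time, then sends it an interact message, guarded by a next-tick retrigger delay.
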(event EventBeginPlay
  (if (Variables|Default|GetbUpdateOnTick)
    (Components|Tick|SetComponentTickEnabled true)
    (else
      (Utilities|Time|SetTimerbyFunctionName 0 "TraceForInteract" (Variables|Default|GetUpdateFrequencey) true))))

(event EventTick
  (params (DeltaSeconds :type Float%20%28single-precision%29))
  (CallFunction|TraceforInteract))

(fn GetTraceLocactions
  (bind _returnvalue (Viewport|GetViewportSize))
  (bind _returnvalue_2 (Game|GetPlayerController 0))
  (bind _returnvalue_3 (/ _returnvalue "(X=2.000000,Y=2.000000)"))
  (bind (_worldposition _worlddirection) (Class|GameplayStatics|DeprojectScreentoWorld _returnvalue_2 _returnvalue_3))
  ;[1 1 1] get locaction from screen to player plus interaction distance
  (return _worldposition (+ _worldposition (* (+ (Math|Vector|Distance(Vector) _worldposition (Transformation|GetActorLocation (Components|GetOwner))) (Variables|Default|GetInteractDistance)) _worlddirection))))

(fn TraceforInteract
  (bind (_start _end) (CallFunction|GetTraceLocactions))
  (bind (_outhit _returnvalue) (Collision|LineTraceByChannel _start _end "TraceTypeQuery3" false 0 "None"))
  (if _returnvalue
    (if (!= (.HitActor (Collision|BreakHitResult _outhit)) (Variables|Default|GetCurrentHitActor))
      (Variables|Default|SetPrevouseHitActor (Variables|Default|GetCurrentHitActor))
      (Variables|Default|SetCurrentHitActor (.HitActor (Collision|BreakHitResult _outhit)))
      (Variables|Default|SetbCanSetPrevious true)
      (Variables|Default|SetCurrentHoldDuration 0.0)
      (CallFunction|UpdateInteractState true :!label _label)
      (elif (CallFunction|GetRecheckHit)
        (CallFunction|DisableHitRecheck)
        (goto _label)))
    (elif (Variables|Default|GetbCanSetPrevious)
      (CallFunction|DisableHitRecheck)
      (Utilities|IsValid (Variables|Default|GetCurrentHitActor)
        (:Is%20Valid
          (Variables|Default|SetPrevouseHitActor (Variables|Default|GetCurrentHitActor)))
        (:Is%20Not%20Valid
          (Variables|Default|SetPrevouseHitActor 0)))
      (Variables|Default|SetCurrentHitActor 0)
      (Variables|Default|SetbCanSetPrevious false)
      (Variables|Default|SetCurrentHoldDuration 0.0)
      (CallFunction|UpdateInteractState false))))

(fn UpdateInteractState
  (params (bHit :type Boolean)))

(fn UpdateInteract
  (params (CurrentHoldDuration :type Float%20%28double-precision%29))
  (Variables|Default|SetCurrentHoldDuration CurrentHoldDuration)
  (if (not (Variables|Default|GetbTriggerDelay))
    (if (.ReturnValue (CallFunction|GetCurrentHit))
      (bind _holdtime (Class|BPIInteractOLD|GetInteractHoldTime(Message) (Variables|Default|GetCurrentHitActor)))
      (Variables|Default|SetInteractHoldTimer _holdtime)
      (if (>= (Variables|Default|GetCurrentHoldDuration) (Variables|Default|GetInteractHoldTimer))
        (CallFunction|TriggerInteract)))))

(fn TriggerInteract
  (CallFunction|RetriggerDelay)
  (if (.ReturnValue (CallFunction|GetCurrentHit))
    (Class|BPIInteractOLD|Interact(Message) (Variables|Default|GetCurrentHitActor) (Components|GetOwner))
    (Variables|Default|SetCurrentHoldDuration 0.0)))

(fn RetriggerDelay
  (if (Variables|Default|GetbTriggerDelay)
    (Variables|Default|SetbTriggerDelay false)
    (else
      (Variables|Default|SetbTriggerDelay true)
      (Class|KismetSystemLibrary|SetTimerforNextTick 0 "RetriggerDelay"))))