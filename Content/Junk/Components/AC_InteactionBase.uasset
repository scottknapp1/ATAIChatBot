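; AC_InteactionBase is an interaction base component that exposes hit-tracking state.
; Getters return the current and previous hit actors, each paired with a validity check.
; A RecheckHit flag has a getter plus enable and disable functions.
; The graphs contain no tracing and never assign the hit actors.
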(fn GetCurrentHit
  (bind _currenthitactor (Variables|Hit|GetCurrentHitActor))
  (return (Utilities|IsValid _currenthitactor) _currenthitactor))

(fn GetPreviousHit
  (bind _prevousehitactor (Variables|Hit|GetPrevouseHitActor))
  (return (Utilities|IsValid _prevousehitactor) _prevousehitactor))

(fn GetRecheckHit
  (return (Variables|Hit|GetbRecheckHit)))

(fn EnableHitRecheck
  (Variables|Hit|SetbRecheckHit true))

(fn DisableHitRecheck
  (Variables|Hit|SetbRecheckHit false))